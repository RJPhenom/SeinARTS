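; SAFI_UNIT_Depr is a Blueprint interface for game units, with a name suffix suggesting it is deprecated.
; It declares selection and queued selection, orders, cloak and reveal, target exchange, damage with penetration and angle, and placement.
; Getters expose player owner, unit instance data, and ammo, HP and MF as values and percentages.
; All functions are stubs that are empty or return defaults, leaving behavior to implementers.
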(fn Select
  (return false 0))

(fn QueueSelect
  (return false 0))

(fn Deselect)

(fn DequeueSelect)

(fn Order
  (params (Target :type Actor%20Object%20Reference) (Position :type Vector))
  (return false))

(fn GetPlayerOwner
  (return 0))

(fn GetUnitData
  (return 0 ""))

(fn Cloak)

(fn Reveal)

(fn ReceiveTarget
  (params (Target :type Actor%20Object%20Reference) (IsOrder :type Boolean)))

(fn RemoveTarget
  (params (Target :type Actor%20Object%20Reference)))

(fn ProvideTarget
  (params (Requestor :type Actor%20Object%20Reference))
  (return 0))

(fn GetAmmo
  (return 0.0))

(fn GetAmmo%
  (return 0.0))

(fn GetHP
  (return 0.0))

(fn GetHP%
  (return 0.0))

(fn GetMF
  (return 0.0))

(fn GetMF%
  (return 0.0))

(fn TakeDmg
  (params (Dmg :type Float%20%28double-precision%29) (Penetration :type Float%20%28double-precision%29) (Angle :type Vector)))

(fn Place
  (params (Position :type Vector) (Rotation :type Rotator)))