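; SAF_CAMERA is a camera pawn that pans, orbits, zooms and can follow a target unit.
; Panning clears the follow target and applies yaw-relative movement input at a normal or Shift speed, consumed manually to set location.
; Rotation turns the actor and zoom slides the camera along local X, using ReverseSmoothClamp for pitch and zoom limits.
; GetBoundedLocation only adds the offset, so panning is unbounded.
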(event EventBeginPlay
  (CallFunction|ResetCamera)
  (Variables|Default|SetMoveSpeed (Variables|Default|GetBaseMoveSpeed)))

(event EventTick
  (params (DeltaSeconds :type Float%20%28single-precision%29))
  (bind _followtarget (Variables|Default|GetFollowTarget))
  ;[0.15 0.15 0.15 0.5] Handles unit follow camera, if set
  (Utilities|IsValid _followtarget
    (:Is%20Valid
      (Transformation|SetActorLocation (Transformation|GetActorLocation _followtarget) false false))))

(fn ConstructionScript)

(fn GetBoundedLocation
  (params (Update%20Vector :type Vector))
  (return (+ Update%20Vector (Transformation|GetActorLocation))))

(fn ToggleSpeed
  (params (Shift :type Boolean))
  (if Shift
    (Variables|Default|SetMoveSpeed (Variables|Default|GetShiftMoveSpeed))
    (else
      (Variables|Default|SetMoveSpeed (Variables|Default|GetBaseMoveSpeed)))))

(fn PanCamera
  (params (Input :type Vector%202D%20Structure))
  (bind _yaw (Utilities|CameraYaw))
  (bind _movespeed (Variables|Default|GetMoveSpeed))
  (Variables|Default|SetFollowTarget 0)
  (Utilities|FlowControl|Sequence
    (:then_0
      (Pawn|Input|AddMovementInput (Utilities|PanRightVector _yaw) (* (.x Input) _movespeed) false))
    (:then_1
      (Pawn|Input|AddMovementInput (Utilities|PanForwardVector _yaw) (* _movespeed (.y Input)) false))
    (:then_2
      (bind _returnvalue (Class|Pawn|ConsumeMovementInputVector))
      (bind _returnvalue_2 (CallFunction|GetBoundedLocation _returnvalue))
      (Transformation|SetActorLocation _returnvalue_2 false false))))

(fn RotateCamera
  (params (Input :type Vector%202D%20Structure))
  (bind _pitch (Utilities|CameraPitch))
  (bind _yaw (Utilities|CameraYaw))
  (bind _rotationspeed (Variables|Default|GetRotationSpeed))
  (bind _result (CallFunction|ReverseSmoothClamp _pitch (+ _pitch (* (.y Input) _rotationspeed -1.0)) (Variables|Default|GetMinAngle) (Variables|Default|GetMaxAngle)))
  (Transformation|SetActorRotation (Math|Rotator|MakeRotator 0.0 _result (Math|Float|Lerp _yaw (+ _yaw (* (.x Input) _rotationspeed)) 0.5))))

(fn ZoomCamera
  (params (Input :type Float%20%28double-precision%29))
  (bind _camera (Variables|Default|GetCamera))
  (bind _camera_2 (Variables|Default|GetCamera))
  (bind _relativelocation (Variables|/Script/Engine.SceneComponent|GetRelativeLocation _camera))
  (bind _result (CallFunction|ReverseSmoothClamp (.x _relativelocation) (+ (.x _relativelocation) (* Input (Variables|Default|GetZoomSpeed) -1.0)) (Variables|Default|GetMinZoom) (Variables|Default|GetMaxZoom)))
  (Transformation|SetRelativeLocation _camera_2 (Math|Vector|MakeVector (Math|Float|Lerp _result (.x (Variables|/Script/Engine.SceneComponent|GetRelativeLocation _camera_2)) 0.5) 0.0 0.0) false false))

(fn ResetCamera
  (Transformation|SetActorRotation (Math|Rotator|MakeRotator 0.0 (Variables|Default|GetDefaultAngle) 0.0))
  (Transformation|SetRelativeLocation (Variables|Default|GetCamera) (Math|Vector|MakeVector (Variables|Default|GetMaxZoom) 0.0 0.0) false false))