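; Player controller for the SeinARTS Framework RTS, routing Enhanced Input to camera, selection, orders and debug pings.
; SAF_CAMERA handles movement, while SAF_HUD draws the selection marquee.
; Units are queued, then selected through interface messages, with marquee picks filtered by player and Shift preserving friendly selections.
; Cursor traces drive move orders and per-tick squad position decals, and placement mode swaps input mapping contexts.
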(event Custom|ReceivePlacement
  (params (PlacementActor :type Actor%20Object%20Reference))
  (bind _returnvalue (PlayerController|LocalPlayerSubsystems|GetEnhancedInputLocalPlayerSubsystem))
  (Variables|Default|SetPlacementActor PlacementActor)
  (Input|RemoveMappingContext _returnvalue "/SeinARTS_Framework/Blueprints/Input/SAF_IMAP.SAF_IMAP" "(bIgnoreAllPressedKeysUntilRelease=True,bForceImmediately=False,bNotifyUserSettings=False)")
  (Input|AddMappingContext _returnvalue "/SeinARTS_Framework/Blueprints/Input/Placement/SAF_IMAP_Placement.SAF_IMAP_Placement" 0 "(bIgnoreAllPressedKeysUntilRelease=True,bForceImmediately=False,bNotifyUserSettings=False)"))

(event Custom|IssueOrder
  (bind (_worldlocation _worlddirection) (Game|Player|ConvertMouseLocationToWorldSpace))
  (bind _outhit (Collision|LineTraceByChannel _worldlocation (* _worlddirection 1e+06) "TraceTypeQuery1" false 0 "None"))
  (for _array_element (Variables|Default|GetSelection)
    (bind _result (Class|SAFIUNITDepr|Order(Message) _array_element 0 (.Location (Collision|BreakHitResult _outhit))))
    (if _result
      (Rendering|Debug|DrawDebugString (.Location (Collision|BreakHitResult _outhit)) "Move here!" 0 "(R=0.000000,G=1.000000,B=0.000000,A=1.000000)" 2.0))))

(event Custom|EndPlacement
  (bind _returnvalue (PlayerController|LocalPlayerSubsystems|GetEnhancedInputLocalPlayerSubsystem))
  (Input|RemoveMappingContext _returnvalue "/SeinARTS_Framework/Blueprints/Input/Placement/SAF_IMAP_Placement.SAF_IMAP_Placement" "(bIgnoreAllPressedKeysUntilRelease=True,bForceImmediately=False,bNotifyUserSettings=False)")
  (Input|AddMappingContext _returnvalue "/SeinARTS_Framework/Blueprints/Input/SAF_IMAP.SAF_IMAP" 0 "(bIgnoreAllPressedKeysUntilRelease=True,bForceImmediately=False,bNotifyUserSettings=False)")
  (Class|SAFIUNITDepr|Place(Message) (Variables|Default|GetPlacementActor) "0, 0, 0" "0, 0, 0")
  (Variables|Default|SetPlacementActor 0))

(event Input|EnhancedActionEvents|EnhancedInputActionSAF_IA-Shift
  (params (ActionValue :type Boolean) (ElapsedSeconds :type Float%20%28double-precision%29) (TriggeredSeconds :type Float%20%28double-precision%29) (InputAction :type Input%20Action%20Object%20Reference :default "/SeinARTS_Framework/Blueprints/Input/SAF_IA-Shift.SAF_IA-Shift"))
  ;[0.15 0.15 0.15 0.5] Camera Controls
  (:Started
    (Default|ToggleSpeed (Variables|SAFReferences|GetSAF_CAMERA) ActionValue :!label _label))
  (:Canceled
    (goto _label))
  (:Completed
    (goto _label)))

(event Input|EnhancedActionEvents|EnhancedInputActionSAF_IA-Pan
  (params (ActionValue :type Vector%202D%20Structure) (ElapsedSeconds :type Float%20%28double-precision%29) (TriggeredSeconds :type Float%20%28double-precision%29) (InputAction :type Input%20Action%20Object%20Reference :default "/SeinARTS_Framework/Blueprints/Input/SAF_IA-Pan.SAF_IA-Pan"))
  ;[0.15 0.15 0.15 0.5] Camera Controls
  (Default|PanCamera (Variables|SAFReferences|GetSAF_CAMERA) ActionValue))

(event Input|EnhancedActionEvents|EnhancedInputActionSAF_IA-Rotate
  (params (ActionValue :type Vector%202D%20Structure) (ElapsedSeconds :type Float%20%28double-precision%29) (TriggeredSeconds :type Float%20%28double-precision%29) (InputAction :type Input%20Action%20Object%20Reference :default "/SeinARTS_Framework/Blueprints/Input/SAF_IA-Rotate.SAF_IA-Rotate"))
  ;[0.15 0.15 0.15 0.5] Camera Controls
  (Default|RotateCamera (Variables|SAFReferences|GetSAF_CAMERA) ActionValue))

(event Input|EnhancedActionEvents|EnhancedInputActionSAF_IA-Zoom
  (params (ActionValue :type Float%20%28double-precision%29) (ElapsedSeconds :type Float%20%28double-precision%29) (TriggeredSeconds :type Float%20%28double-precision%29) (InputAction :type Input%20Action%20Object%20Reference :default "/SeinARTS_Framework/Blueprints/Input/SAF_IA-Zoom.SAF_IA-Zoom"))
  ;[0.15 0.15 0.15 0.5] Camera Controls
  (Default|ZoomCamera (Variables|SAFReferences|GetSAF_CAMERA) ActionValue))

(event Input|EnhancedActionEvents|EnhancedInputActionSAF_IA-Reset
  (params (ActionValue :type Boolean) (ElapsedSeconds :type Float%20%28double-precision%29) (TriggeredSeconds :type Float%20%28double-precision%29) (InputAction :type Input%20Action%20Object%20Reference :default "/SeinARTS_Framework/Blueprints/Input/SAF_IA-Reset.SAF_IA-Reset"))
  ;[0.15 0.15 0.15 0.5] Camera Controls
  (:Completed
    (Default|ResetCamera (Variables|SAFReferences|GetSAF_CAMERA))))

(event Input|EnhancedActionEvents|EnhancedInputActionSAF_IA-Follow
  (params (ActionValue :type Boolean) (ElapsedSeconds :type Float%20%28double-precision%29) (TriggeredSeconds :type Float%20%28double-precision%29) (InputAction :type Input%20Action%20Object%20Reference :default "/SeinARTS_Framework/Blueprints/Input/SAF_IA-Follow.SAF_IA-Follow"))
  ;[0.15 0.15 0.15 0.5] Camera Controls
  (:Canceled
    (Utilities|IsValid (Variables|Default|GetActiveUnit) :!label _label
      (:Is%20Valid
        (Variables|/SeinARTS_Framework/Blueprints/SAF_CAMERA.SAF_CAMERA_C|SetFollowTarget (Variables|SAFReferences|GetSAF_CAMERA) 0))))
  (:Completed
    (goto _label)))

(event Input|EnhancedActionEvents|EnhancedInputActionSAF_IA-Select
  (params (ActionValue :type Boolean) (ElapsedSeconds :type Float%20%28double-precision%29) (TriggeredSeconds :type Float%20%28double-precision%29) (InputAction :type Input%20Action%20Object%20Reference :default "/SeinARTS_Framework/Blueprints/Input/SAF_IA-Select.SAF_IA-Select"))
  (bind _saf_hud (Variables|SAFReferences|GetSAF_HUD))
  ;[0.15 0.15 0.15 0.5] Select Input Handling: Mouse delta tracking is handled in the SAF_HUD Class, which is responsible for drawing the marquee for drag selecting. The SAF_HUD then returns results to the receiver event below.
  (:Triggered
    (bind _returnvalue (CallFunction|GetMouseVector2D))
    (bind _output_get (Variables|Default|SetCurrentSelectPosition _returnvalue))
    (Default|UpdateMarquee _saf_hud _output_get))
  (:Started
    (bind _returnvalue_2 (CallFunction|GetMouseVector2D))
    (bind _output_get_2 (Variables|Default|SetInitialSelectPosition _returnvalue_2))
    (Default|StartMarquee _saf_hud _output_get_2))
  (:Canceled
    (bind _marqueedrawn (Default|EndMarquee _saf_hud :!label _label))
    (Selection|UpdateSelection _marqueedrawn))
  (:Completed
    (goto _label)))

(event Input|EnhancedActionEvents|EnhancedInputActionSAF_IA-Order
  (params (ActionValue :type Boolean) (ElapsedSeconds :type Float%20%28double-precision%29) (TriggeredSeconds :type Float%20%28double-precision%29) (InputAction :type Input%20Action%20Object%20Reference :default "/SeinARTS_Framework/Blueprints/Input/SAF_IA-Order.SAF_IA-Order"))
  ;[0.15 0.15 0.15 0.5] Ping Handling tracks mouse cursor delta locally, since we are not adding anything specific to the Event Draw HUD method.
  (:Triggered
    (bind _returnvalue (CallFunction|GetMouseVector2D))
    (bind _output_get (Variables|Default|SetCurrentOrderPosition _returnvalue))
    (Utilities|2DLengthCheck (stale _output_get_2) _output_get 5.0))
  (:Started
    (bind _returnvalue_2 (CallFunction|GetMouseVector2D))
    (bind _output_get_2 (Variables|Default|SetInitialOrderPosition _returnvalue_2)))
  (:Canceled
    (CallFunction|IssueOrder :!label _label))
  (:Completed
    (goto _label)))

(event Input|EnhancedActionEvents|EnhancedInputActionSAF_IA-Ping
  (params (ActionValue :type Boolean) (ElapsedSeconds :type Float%20%28double-precision%29) (TriggeredSeconds :type Float%20%28double-precision%29) (InputAction :type Input%20Action%20Object%20Reference :default "/SeinARTS_Framework/Blueprints/Input/SAF_IA-Ping.SAF_IA-Ping"))
  (bind (_worldlocation _worlddirection) (Game|Player|ConvertMouseLocationToWorldSpace))
  ;[0.15 0.15 0.15 0.5] Ping Handling tracks mouse cursor delta locally, since we are not adding anything specific to the Event Draw HUD method.
  (:Started
    (bind _returnvalue (CallFunction|GetMouseVector2D))
    (bind _output_get (Variables|Default|SetInitialPingPosition _returnvalue)))
  (:Canceled
    (bind _returnvalue_2 (CallFunction|GetMouseVector2D :!label _label))
    (bind _output_get_2 (Variables|Default|SetCurrentPingPosition _returnvalue_2))
    (Utilities|2DLengthCheck _output_get _output_get_2 5.0
      (:Lesser
        (Development|PrintString "Ping!")
        (bind _outhit (Collision|LineTraceByChannel _worldlocation (* _worlddirection 1e+05) "TraceTypeQuery1" false 0 "None"))
        (Rendering|Debug|DrawDebugString (.location _outhit) "Ping!" 0 "(R=1.000000,G=0.002830,B=0.898389,A=1.000000)" 2.0))))
  (:Completed
    (goto _label)))

(event EventBeginPlay
  (bind _returnvalue (PlayerController|LocalPlayerSubsystems|GetEnhancedInputLocalPlayerSubsystem))
  (Utilities|FlowControl|Sequence
    (:then_0
      ;[0.15 0.15 0.15 0.5] Init Input Sys
      (Utilities|IsValid _returnvalue
        (:Is%20Valid
          (Input|AddMappingContext _returnvalue "/SeinARTS_Framework/Blueprints/Input/SAF_IMAP.SAF_IMAP" 0 "(bIgnoreAllPressedKeysUntilRelease=True,bForceImmediately=False,bNotifyUserSettings=False)"))))
    (:then_1
      (Variables|Default|SetbShowMouseCursor true))
    (:then_2
      ;[0.15 0.15 0.15 0.5] Init SeinARTS Framework References
      (Variables|SAFReferences|SetSAF_CAMERA (.AsSAF%20CAMERA (Utilities|Casting|CastToSAF_CAMERA (Pawn|GetControlledPawn))))
      (Variables|SAFReferences|SetSAF_HUD (.AsSAF%20HUD (Utilities|Casting|CastToSAF_HUD (HUD|GetHUD)))))))

(event EventMarqueeSelect
  (params (Targets :type Array%20of%20Actor%20Object%20References))
  (Selection|ClearSelectionQueue)
  (bind _outselection (CallFunction|FilterSelectionbyPlayer Targets (Variables|Default|GetPlayerID)))
  (for _array_element _outselection
    (Utilities|AttemptQueuedSelection _array_element
      (:Failed
        (Development|PrintString "Hello" true true "(R=1.000000,G=0.000000,B=0.042461,A=1.000000)")))))

(event EventSingleSelect
  (params (Target :type Actor%20Object%20Reference))
  (Selection|ClearSelectionQueue)
  (Utilities|AttemptQueuedSelection Target))

(event EventTick
  (params (DeltaSeconds :type Float%20%28single-precision%29))
  (Rendering|Debug|DrawDebugPoint "0, 0, 0" 5.0 "(R=1.000000,G=0.000000,B=0.515852,A=1.000000)" 0.0)
  (for _array_element (Variables|Default|GetSelection)
    (Utilities|IsValid _array_element
      (:Is%20Valid
        (bind _assaf_squad (Utilities|Casting|CastToSAF_Squad _array_element))
        (bind _position (Utilities|TraceMouseUnderCursor)
          (:%20
            (Default|DrawPositionDecals _assaf_squad _position)))))))

(fn ConstructionScript)

(fn GetMouseVector2D
  (bind (_locationx _locationy) (Game|Player|GetMousePosition))
  (return (Math|Vector2D|MakeVector2D _locationx _locationy)))

(fn GetPlacementActive
  (return (Utilities|IsValid (Variables|Default|GetPlacementActor))))

(fn GetSelection
  (return (Variables|Default|GetSelection)))

(fn SetSelection
  (params (Select :type Array%20of%20Actor%20Object%20References))
  (Utilities|FlowControl|Sequence
    (:then_0
      (Selection|ClearSelection))
    (:then_1
      (for _array_element Select
        (bind _result (Class|SAFIUNITDepr|Select(Message) _array_element))
        (if (not _result)
          (Development|PrintString (Utilities|String|Append "'SetSelection' method failed on one or more members: " (Utilities|GetDisplayName _array_element) " failed to select or does not implement the required interface.")))))
    (:then_2
      (Variables|Default|SetSelection Select))))

(fn UpdateSelection
  (params (MarqueeDrawn :type Boolean))
  (Utilities|IsShiftDown
    (:True
      (Utilities|IsMySelectionFriendly
        (:True
          _)
        (:False
          (Selection|ClearSelection :!label _label))))
    (:False
      (goto _label)))
  (if MarqueeDrawn
    (Selection|MarqueeSelect)
    (else
      (Selection|SingleSelect)))
  (Selection|ClearSelectionQueue)
  (Selection|LogSelection))

(fn ClearSelection
  (bind _selection (Variables|Default|GetSelection))
  (Utilities|FlowControl|Sequence
    (:then_0
      (for _array_element _selection
        (Class|SAFIUNITDepr|Deselect(Message) _array_element)))
    (:then_1
      (Utilities|Array|Clear _selection))))

(fn ClearSelectionQueue
  (bind _selectionqueue (Variables|Default|GetSelectionQueue))
  (Utilities|FlowControl|Sequence
    (:then_0
      (for _array_element _selectionqueue
        (Class|SAFIUNITDepr|DequeueSelect(Message) _array_element)))
    (:then_1
      (Utilities|Array|Clear _selectionqueue))))

(fn LogSelection
  (Development|PrintString (Utilities|String|Append "Selection logged: " (Utilities|String|ToString(Integer) (Utilities|Array|Length (Variables|Default|GetSelection))) " units.")))

(fn SingleSelect
  (Utilities|AttemptSelection (Utilities|Array|Get(acopy) (Variables|Default|GetSelectionQueue))))

(fn MarqueeSelect
  (bind _outselection (CallFunction|FilterSelectionbyPlayer (Variables|Default|GetSelectionQueue) (Variables|Default|GetPlayerID)))
  (for _array_element _outselection
    (Utilities|AttemptSelection _array_element
      (:Selected
        (Utilities|Array|AddUnique (Variables|Default|GetSelection) _array_element)))))

(fn SendOrders
  (params (OrderTarget :type %20Object%20Reference) (OrderPosition :type Vector))
  (Utilities|IsMySelectionFriendly
    (:True
      (for _array_element (Variables|Default|GetSelection)
        (Class|SAFIUNITDepr|Order(Message) _array_element 0 "0, 0, 0")))))

(fn Select
  (params (Target :type Actor%20Object%20Reference))
  (if (Utilities|DoesObjectImplementInterface Target "/SeinARTS_Framework/Blueprints/Interfaces/SAFI_UNIT_Depr.SAFI_UNIT_Depr_C")
    (bind (_result _unitselected) (Class|SAFIUNITDepr|Select(Message) Target))
    (if _result
      (Utilities|Array|AddUnique (Variables|Default|GetSelection) _unitselected)
      (return true)
      (else
        _)))
  (return false))

(fn QueueSelect
  (params (Target :type Actor%20Object%20Reference))
  (if (Utilities|DoesObjectImplementInterface Target "/SeinARTS_Framework/Blueprints/Interfaces/SAFI_UNIT_Depr.SAFI_UNIT_Depr_C")
    (bind (_result _unitqueueselected) (Class|SAFIUNITDepr|QueueSelect(Message) Target))
    (if _result
      (Utilities|Array|AddUnique (Variables|Default|GetSelectionQueue) _unitqueueselected)
      (return true)
      (else
        _)))
  (return false))

(fn GetActiveUnit
  (return (Variables|Default|GetActiveUnit)))

(fn GetActiveUnitData
  (bind _data (Class|SAFIUNITDepr|GetUnitData(Message) (Variables|Default|GetActiveUnit)))
  (return _data))

(fn GetSelectionData
  (for _array_element (Variables|Default|GetSelection)
    (bind _data (Class|SAFIUNITDepr|GetUnitData(Message) _array_element))
    (Utilities|Array|Add (LocalVariables|GetCummulativeData) _data))
  (return (LocalVariables|GetCummulativeData)))