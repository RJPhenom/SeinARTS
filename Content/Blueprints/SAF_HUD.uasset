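; SAF_HUD is the SeinARTS Framework HUD that draws the drag-select marquee and reports selection to SAF_PC.
; StartMarquee and UpdateMarquee store the drag points and rectangle dimensions.
; While active, DrawHUD compares drag length to a threshold each frame, sending either pawns inside the drawn rectangle or the actor under the cursor.
; EndMarquee resets state and returns whether the drag qualified as a marquee.
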(event Custom|StartMarquee
  (params (Start :type Vector%202D%20Structure))
  ;[0.15 0.15 0.15 0.5] Event Handling / Receivers for Selection Rect Drawing
  (CallFunction|BeginMarquee Start))

(event Custom|UpdateMarquee
  (params (End :type Vector%202D%20Structure))
  ;[0.15 0.15 0.15 0.5] Event Handling / Receivers for Selection Rect Drawing
  (bind _output_get (Variables|Default|SetEnd End))
  (bind (_width _height _x _y) (CallFunction|GetRectParams (Variables|Default|GetStart) _output_get))
  (Variables|Default|SetWidth _width)
  (Variables|Default|SetHeight _height)
  (Variables|Default|SetX _x)
  (Variables|Default|SetY _y))

(event EventBeginPlay
  ;[0.15 0.15 0.15 0.5] Init SeinARTS Framework References
  (Variables|SAFReferences|SetSAF_PC (.AsSAF%20PC (Utilities|Casting|CastToSAF_PC (Game|GetPlayerController 0)))))

(event EventDrawHUD
  (params (SizeX :type Integer) (SizeY :type Integer))
  (bind _saf_pc (Variables|SAFReferences|GetSAF_PC))
  ;[0.15 0.15 0.15 0.5] Orders draw routines
  (Utilities|FlowControl|Sequence
    (:then_0
      ;[0.15 0.15 0.15 0.5] Draw Drag-Select Marquee
      ;;[0.15 0.15 0.15 0.5] Checks if we are drawing, and if the delta between Mouse Start and Mouse End is great enough to draw a marquee (otherwise handle as a single-select)
      (if (Variables|Default|GetDrawMarquee)
        (Utilities|2DLengthCheck (Variables|Default|GetStart) (Variables|Default|GetEnd) (Variables|Default|GetMarqueeThreshold)
          (:Greater
            (HUD|DrawRect (Variables|Default|GetRect%20Color) (Variables|Default|GetX) (Variables|Default|GetY) (Variables|Default|GetWidth) (Variables|Default|GetHeight))
            (bind _output_get (Variables|Default|SetSelectResults (Class|HUD|GetActorsinSelectionRectangle "/Script/Engine.Pawn" (Variables|Default|GetStart) (Variables|Default|GetEnd) true false)))
            (Class|SAFIPLAYERDepr|ReceiveMarqueeSelect(Message) _saf_pc _output_get))
          (:Lesser
            (Class|SAFIPLAYERDepr|ReceiveSingleSelect(Message) _saf_pc (.HitActor (Collision|BreakHitResult (.HitResult (Game|Player|GetHitResultUnderCursorbyChannel (Variables|SAFReferences|GetSAF_PC) "TraceTypeQuery1" true)))))))))))

(fn ConstructionScript)

(fn GetRectParams
  (params (Start :type Vector%202D%20Structure) (End :type Vector%202D%20Structure))
  (return (- (.x End) (.x Start)) (- (.y End) (.y Start)) (.x Start) (.y Start)))

(fn BeginMarquee
  (params (Start :type Vector%202D%20Structure))
  (Variables|Default|SetStart Start)
  (Variables|Default|SetDrawMarquee true))

(fn EndMarquee
  ;[0.15 0.15 0.15 0.5] Check (and output) if we drew a rect. This is important for determining single-select.
  (Utilities|2DLengthCheck (Variables|Default|GetStart) (Variables|Default|GetEnd) (Variables|Default|GetMarqueeThreshold)
    (:Greater
      (LocalVariables|SetWasMarqueeDrawn true))
    (:Lesser
      (LocalVariables|SetWasMarqueeDrawn false)))
  (Variables|Default|SetDrawMarquee false)
  (Variables|Default|SetStart "")
  (Variables|Default|SetEnd "")
  (Variables|Default|SetWidth 0.0)
  (Variables|Default|SetHeight 0.0)
  (Variables|Default|SetX 0.0)
  (Variables|Default|SetY 0.0)
  (Utilities|Array|Clear (Variables|Default|GetSelectResults))
  (return (LocalVariables|GetWasMarqueeDrawn)))