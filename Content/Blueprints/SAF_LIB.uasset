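; SAF_LIB is a function library of math and unit-selection ownership helpers.
; SmoothClamp clamps the midpoint of two values to a range, and ReverseSmoothClamp calls it with the bounds swapped.
; IsSelectionFriendly compares only the first element's owner to a player ID, returning true if that element is invalid.
; FilterSelectionByPlayer keeps elements whose owner, queried through GetPlayerOwnerMessage, matches the ID.
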(fn SmoothClamp
  (params (A :type Float%20%28double-precision%29) (B :type Float%20%28double-precision%29) (Min :type Float%20%28double-precision%29) (Max :type Float%20%28double-precision%29))
  (return (Math|Float|Clamp(Float) (Math|Float|Lerp A B 0.5) Min Max)))

(fn ReverseSmoothClamp
  (params (A :type Float%20%28double-precision%29) (B :type Float%20%28double-precision%29) (Min :type Float%20%28double-precision%29) (Max :type Float%20%28double-precision%29))
  (bind _result (CallFunction|SmoothClamp A B Max Min))
  (return _result))

(fn IsSelectionFriendly
  (params (Selection :type Array%20of%20Actor%20Object%20References) (PlayerID :type Integer))
  (bind _output (Utilities|Array|Get(acopy) Selection))
  (Utilities|IsValid _output
    (:Is%20Valid
      (bind _owner (Class|SAFIUNITDepr|GetPlayerOwner(Message) _output))
      (return (== _owner PlayerID)))
    (:Is%20Not%20Valid
      (return true))))

(fn FilterSelectionbyPlayer
  (params (Selection :type Array%20of%20Actor%20Object%20References) (PlayerID :type Integer))
  (for _array_element Selection
    (bind _owner (Class|SAFIUNITDepr|GetPlayerOwner(Message) _array_element))
    (if (== _owner PlayerID)
      (Utilities|Array|Add (LocalVariables|GetFilteredSelection) _array_element)))
  (return (LocalVariables|GetFilteredSelection)))