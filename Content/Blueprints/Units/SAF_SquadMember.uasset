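; Squad member actor belonging to a parent Unit, which it forwards selection, owner queries and targets to.
; InitSquadMember sizes the view, detection and weapon spheres and sets HP from SquadMemberData, destroying the actor if that is missing.
; Weapon-range overlaps add or remove Unit targets, detection overlaps send a reveal message, and cover events track cover objects.
; Stat getters, unit data, orders and target provision are stubs.
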(event OnComponentBeginOverlap(WeaponRange)
  (params (OverlappedComponent :type Primitive%20Component%20Object%20Reference) (OtherActor :type Actor%20Object%20Reference) (OtherComp :type Primitive%20Component%20Object%20Reference) (OtherBodyIndex :type Integer) (bFromSweep :type Boolean) (SweepResult :type Hit%20Result%20Structure%20%28by%20ref%29))
  (Utilities|IsUnit OtherActor
    (:True
      (Default|ReceiveTarget (Variables|Data|GetUnit) OtherActor false))))

(event OnComponentEndOverlap(WeaponRange)
  (params (OverlappedComponent :type Primitive%20Component%20Object%20Reference) (OtherActor :type Actor%20Object%20Reference) (OtherComp :type Primitive%20Component%20Object%20Reference) (OtherBodyIndex :type Integer))
  (Utilities|IsUnit OtherActor
    (:True
      (Default|RemoveTarget (Variables|Data|GetUnit) OtherActor))))

(event OnComponentBeginOverlap(DetectionRange)
  (params (OverlappedComponent :type Primitive%20Component%20Object%20Reference) (OtherActor :type Actor%20Object%20Reference) (OtherComp :type Primitive%20Component%20Object%20Reference) (OtherBodyIndex :type Integer) (bFromSweep :type Boolean) (SweepResult :type Hit%20Result%20Structure%20%28by%20ref%29))
  (Class|SAFIUNITDepr|Reveal(Message) OtherActor))

(event Custom|EnterCover
  (params (CoverObject :type Actor%20Object%20Reference) (Class :type SAFEnum_CoverClass%20Enum :default "NewEnumerator4") (Direction :type Vector))
  (Utilities|Array|AddUnique (Variables|Default|GetCoverObjects) CoverObject)
  (Utilities|Array|AddUnique (Variables|Default|GetCoverDirections) Direction)
  (Development|PrintString (Utilities|String|Append (Utilities|GetDisplayName self) " entered cover: " (Utilities|String|ToString(Byte) Class)) true true "(R=0.000000,G=1.000000,B=0.000000,A=1.000000)"))

(event Custom|ExitCover
  (params (CoverObject :type Actor%20Object%20Reference) (Class :type SAFEnum_CoverClass%20Enum :default "NewEnumerator4"))
  (Utilities|Array|RemoveItem (Variables|Default|GetCoverObjects) CoverObject)
  (Development|PrintString (Utilities|String|Append (Utilities|GetDisplayName self) " exited cover: " (Utilities|String|ToString(Byte) Class)) true true "(R=1.000000,G=0.450772,B=0.000000,A=1.000000)"))

(event EventBeginPlay)

(event Collision|EventActorBeginOverlap
  (params (OtherActor :type Actor%20Object%20Reference)))

(event EventTick
  (params (DeltaSeconds :type Float%20%28single-precision%29)))

(fn ConstructionScript)

(fn InitSquadMember
  (bind _squadmemberdata (Variables|Data|GetSquadMemberData))
  ;[0.15 0.15 0.15 0.5] Debug
  (Utilities|IsValid (Variables|Data|GetSquadMemberData)
    (:Is%20Valid
      ;[0.15 0.15 0.15 0.5] Set Range Sphere Radii
      (Components|Sphere|SetSphereRadius (Variables|Default|GetViewRange) (Variables|/SeinARTS_Framework/Blueprints/Data/SAFD_SquadMember.SAFD_SquadMember_C|GetFoV _squadmemberdata) true)
      (Components|Sphere|SetSphereRadius (Variables|Default|GetDetectionRange) (Variables|/SeinARTS_Framework/Blueprints/Data/SAFD_SquadMember.SAFD_SquadMember_C|GetDetectRadius _squadmemberdata) true)
      (Components|Sphere|SetSphereRadius (Variables|Default|GetWeaponRange) (Variables|/SeinARTS_Framework/Blueprints/Data/SAFD_Weapon.SAFD_Weapon_C|GetRange (Variables|/SeinARTS_Framework/Blueprints/Data/SAFD_SquadMember.SAFD_SquadMember_C|GetDefaultWeapon _squadmemberdata)) true)
      ;[0.15 0.15 0.15 0.5] Set runtime HP to max
      (Variables|Default|SetHP (Variables|/SeinARTS_Framework/Blueprints/Data/SAFD_SquadMember.SAFD_SquadMember_C|GetHP (Variables|Data|GetSquadMemberData))))
    (:Is%20Not%20Valid
      (Development|PrintString "[ERROR] Failed to initialize SAF_SquadMember. Data was null at time of initialization." true true "(R=1.000000,G=0.000000,B=0.000000,A=1.000000)" 3.0)
      (Actor|DestroyActor))))

(fn GetAmmo
  (return 0.0))

(fn GetAmmo%
  (return 0.0))

(fn GetHP
  (return 0.0))

(fn GetHP%
  (return 0.0))

(fn GetMF
  (return 0.0))

(fn GetMF%
  (return 0.0))

(fn GetPlayerOwner
  (bind _owner (Default|GetPlayerOwner (Variables|Data|GetUnit)))
  (return _owner))

(fn GetUnitData
  (return 0 ""))

(fn Order
  (params (Target :type Actor%20Object%20Reference) (Position :type Vector :default "0, 0, 0"))
  (return false))

(fn ProvideTarget
  (params (Requestor :type Actor%20Object%20Reference))
  (return 0))

(fn QueueSelect
  (bind _unit (Variables|Data|GetUnit))
  (bind _output_get (Variables|/SeinARTS_Framework/Blueprints/Units/SAF_Squad.SAF_Squad_C|SetSelectQueued _unit (Variables|/SeinARTS_Framework/Blueprints/Units/SAF_Squad.SAF_Squad_C|GetSelectable _unit)))
  (return _output_get _unit))

(fn Select
  (bind _unit (Variables|Data|GetUnit))
  (bind _output_get (Variables|/SeinARTS_Framework/Blueprints/Units/SAF_Squad.SAF_Squad_C|SetSelected _unit (Variables|/SeinARTS_Framework/Blueprints/Units/SAF_Squad.SAF_Squad_C|GetSelectable _unit)))
  (return _output_get _unit))