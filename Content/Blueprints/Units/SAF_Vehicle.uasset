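; SAF_Vehicle is a selectable, player-owned vehicle unit that reports ammo, HP and fuel and takes AI move orders.
; The server assigns a GUID instance ID on BeginPlay, and InitVehicle reads unit and vehicle data, though it never sets HP or Fuel.
; Order sends its AI controller to a position, ignoring the target.
; Select and queue-select respect Selectable, with Tick drawing debug labels; ProvideTarget is a stub.
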(event EventBeginPlay
  (Networking|SwitchHasAuthority
    (:Authority
      (Variables|Default|SetInstanceID (Guid|ToString(Guid) (Guid|NewGuid))))))

(event Collision|EventActorBeginOverlap
  (params (OtherActor :type Actor%20Object%20Reference)))

(event EventTick
  (params (DeltaSeconds :type Float%20%28single-precision%29))
  (bind _returnvalue (Transformation|GetActorLocation))
  (if (Variables|Selection|GetSelected)
    (Rendering|Debug|DrawDebugString _returnvalue "Selected!" 0 "(R=0.039546,G=0.665387,B=0.000000,A=1.000000)")
    (elif (Variables|Selection|GetSelectQueued)
      (Rendering|Debug|DrawDebugString _returnvalue "Queued for selection!" 0 "(R=1.000000,G=0.500000,B=0.000000,A=1.000000)"))))

(event EventDeselect
  (Variables|Selection|SetSelected false))

(event EventDequeueSelect
  (Variables|Selection|SetSelectQueued false))

(fn ConstructionScript)

(fn InitVehicle
  (bind _vehicledata (Variables|Data|GetVehicleData))
  ;[0.15 0.15 0.15 0.5] Debug
  (if (and (Utilities|IsValid (Variables|Data|GetUnitData)) (Utilities|IsValid (Variables|Data|GetVehicleData)))
    (Variables|Default|SetReactiveArmour (Variables|/SeinARTS_Framework/Blueprints/Data/SAFD_Vehicle.SAFD_Vehicle_C|GetReactiveArmour _vehicledata))
    (Variables|Default|SetAmmo (Variables|/SeinARTS_Framework/Blueprints/Data/SAFD_Vehicle.SAFD_Vehicle_C|GetHP _vehicledata))
    (Variables|Default|SetAmmo (Variables|/SeinARTS_Framework/Blueprints/Data/SAFD_Unit.SAFD_Unit_C|GetAmmo (Variables|Data|GetUnitData)))
    (else
      (Development|PrintString "[ERROR] Failed to initialize SAF_Vehicle. Data was null at time of initialization." true true "(R=1.000000,G=0.000000,B=0.000000,A=1.000000)" 3.0)
      (Actor|DestroyActor))))

(fn GetAmmo
  (return (Variables|Default|GetAmmo)))

(fn GetAmmo%
  (return (/ (Variables|Default|GetAmmo) (Variables|/SeinARTS_Framework/Blueprints/Data/SAFD_Unit.SAFD_Unit_C|GetAmmo (Variables|Data|GetUnitData)))))

(fn GetHP
  (return (Variables|Default|GetHP)))

(fn GetHP%
  (return (/ (Variables|Default|GetHP) (Variables|/SeinARTS_Framework/Blueprints/Data/SAFD_Vehicle.SAFD_Vehicle_C|GetHP (Variables|Data|GetVehicleData)))))

(fn GetMF
  (return (Variables|Default|GetFuel)))

(fn GetMF%
  (return (/ (Variables|Default|GetFuel) (Variables|/SeinARTS_Framework/Blueprints/Data/SAFD_Vehicle.SAFD_Vehicle_C|GetFuel (Variables|Data|GetVehicleData)))))

(fn GetPlayerOwner
  (return (Variables|Data|GetPlayerOwner)))

(fn GetUnitData
  (return (Variables|Data|GetUnitData) (Variables|Default|GetInstanceID)))

(fn Order
  (params (Target :type Actor%20Object%20Reference) (Position :type Vector :default "0, 0, 0"))
  (AI|Navigation|MovetoLocation (AI|GetAIController self) Position 1.0 true true false true 0)
  (return true))

(fn ProvideTarget
  (params (Requestor :type Actor%20Object%20Reference))
  (return 0))

(fn QueueSelect
  (bind _output_get (Variables|Selection|SetSelectQueued (Variables|Selection|GetSelectable)))
  (return _output_get self))

(fn Select
  (bind _output_get (Variables|Selection|SetSelected (Variables|Selection|GetSelectable)))
  (return _output_get self))