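; SAF_Squad is a squad unit actor that spawns members from SquadData, follows its leader and tracks selection, targets, health, ammo and morale.
; Orders move members through AI controllers into cover or a rotated formation, mirrored when moving behind the leader.
; QueryAreaForCover spaces positions along cover using traces and navmesh projection, a rough prototype flagged for refactoring.
; Debug drawing shows selection state and previews destination positions.
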(event EventBeginPlay
  (Networking|SwitchHasAuthority
    (:Authority
      (Variables|Data|SetInstanceID (Guid|ToString(Guid) (Guid|NewGuid))))
    (:Remote
      _))
  (CallFunction|InitSquad))

(event EventTarget
  (params (Target :type Actor%20Object%20Reference) (IsOrder :type Boolean))
  (if IsOrder
    (Variables|Default|SetActiveTarget Target))
  (Utilities|Array|AddUnique (Variables|Default|GetAllTargets) Target)
  (Development|PrintString (Utilities|String|Append "Target recieved: " (Utilities|GetDisplayName Target) " now in " (Utilities|GetDisplayName self) " targets array.")))

(event EventRemoveTarget
  (params (Target :type Actor%20Object%20Reference))
  (Utilities|Array|RemoveItem (Variables|Default|GetAllTargets) Target)
  (Development|PrintString (Utilities|String|Append "Target removed: " (Utilities|GetDisplayName Target) " no longer in " (Utilities|GetDisplayName self) " targets array.")))

(event EventReveal
  (Rendering|Debug|DrawDebugString (Transformation|GetActorLocation) "Revealed!" 0 "(R=1.000000,G=0.500000,B=0.000000,A=1.000000)" 2.0))

(event EventDeselect
  (Variables|Selection|SetSelected false))

(event EventDequeueSelect
  (Variables|Selection|SetSelectQueued false))

(event EventTick
  (params (DeltaSeconds :type Float%20%28single-precision%29))
  (bind _returnvalue (Transformation|GetActorLocation))
  (bind _returnvalue_2 (Transformation|GetActorLocation))
  (bind _leader_position (Utilities|GetLeaderPosition))
  (bind _leader_position_2 (Utilities|GetLeaderPosition))
  (Transformation|SetActorLocationAndRotation _leader_position (Utilities|GetLeaderRotation))
  (Rendering|Debug|DrawDebugCircle _leader_position (Utilities|GetSpacing) 12 "(R=0.005568,G=0.089347,B=1.000000,A=1.000000)" 0.0 1.0 "0.000000,1.000000,0.000000" "1.000000,0.000000,0.000000")
  (Rendering|Debug|DrawDebugArrow _returnvalue (+ _returnvalue (* (Transformation|GetActorForwardVector) 1e+02)) 1e+01 "(R=0.244792,G=0.094347,B=0.172948,A=1.000000)" 0.0 2.0)
  (Rendering|Debug|DrawDebugArrow _leader_position_2 (+ _leader_position_2 (* (Utilities|GetLeaderForward) 5e+01)) 1e+01 "(R=1.000000,G=0.768009,B=0.000000,A=1.000000)" 0.0 5.0)
  (if (Variables|Selection|GetSelected)
    (Rendering|Debug|DrawDebugString _returnvalue_2 "Selected!" 0 "(R=0.039546,G=0.665387,B=0.000000,A=1.000000)")
    (elif (Variables|Selection|GetSelectQueued)
      (Rendering|Debug|DrawDebugString _returnvalue_2 "Queued for selection!" 0 "(R=1.000000,G=0.500000,B=0.000000,A=1.000000)"))))

(event EventCloak
  (Rendering|Debug|DrawDebugString (Transformation|GetActorLocation) "Cloaked!" 0 "(R=0.000000,G=1.000000,B=0.000000,A=1.000000)" 2.0))

(fn ConstructionScript)

(fn InitSquad
  (bind _squaddata (Variables|Data|GetSquadData))
  ;[0.15 0.15 0.15 0.5] Debug
  (if (and (Utilities|IsValid (Variables|Data|GetUnitData)) (Utilities|IsValid _squaddata))
    (if (Utilities|Array|IsValidIndex (Variables|/SeinARTS_Framework/Blueprints/Data/SAFD_Squad.SAFD_Squad_C|GetSquadMembers _squaddata))
      ;[0.15 0.15 0.15 0.5] Initalization
      (CallFunction|InitPositions)
      (CallFunction|InitSquadMembers)
      (Variables|Default|SetMorale (Variables|/SeinARTS_Framework/Blueprints/Data/SAFD_Squad.SAFD_Squad_C|GetMorale (Variables|Data|GetSquadData)))
      (else
        (Development|PrintString "[ERROR] Failed to initialize SAF_Squad. Squad members array was empty in SquadData." true true "(R=1.000000,G=0.000000,B=0.000000,A=1.000000)" 3.0)
        (Actor|DestroyActor :!label _label)))
    (else
      (Development|PrintString "[ERROR] Failed to initialize SAF_Squad. Data was null at time of initialization." true true "(R=1.000000,G=0.000000,B=0.000000,A=1.000000)" 3.0)
      (goto _label))))

(fn InitSquadMembers
  (for (_array_element _array_index) (Variables|/SeinARTS_Framework/Blueprints/Data/SAFD_Squad.SAFD_Squad_C|GetSquadMembers (Variables|Data|GetSquadData))
    (bind _returnvalue (Game|SpawnActorfromClass "/SeinARTS_Framework/Blueprints/Units/SAF_SquadMember.SAF_SquadMember_C" (Math|Transform|MakeTransform (Utilities|Array|Get(acopy) (Variables|Default|GetPositions) _array_index) (Transformation|GetActorRotation)) "Undefined" "MultiplyWithRoot" 0 _array_element 0 self 0))
    (Utilities|Array|Add (Variables|Data|GetSquadMembers) _returnvalue)))

(fn InitPositions
  (bind _outpositions (CallFunction|PivotPositions (Transformation|GetActorRotation) (Variables|/SeinARTS_Framework/Blueprints/Data/SAFD_Squad.SAFD_Squad_C|GetFormation (Variables|Data|GetSquadData))))
  (for _array_element _outpositions
    (Utilities|Array|Add (LocalVariables|GetInitializedPositions) (+ _array_element (Transformation|GetActorLocation))))
  (bind _output_get (Variables|Default|SetPositions (LocalVariables|GetInitializedPositions)))
  (bind _output_get_2 (Variables|Default|SetPositionDecals _output_get))
  (CallFunction|MoveCharacterstoPositions _output_get_2))

(fn InvertPositions
  (params (InPositions :type Array%20of%20Vectors))
  (if (> (Utilities|Array|Length InPositions) 1)
    (for _array_element InPositions
      (bind _result (Math|Float|NegateFloat (.X (Math|Vector|BreakVector _array_element)))
        (:%20%20
          (bind _result_2 (Math|Float|NegateFloat (.Y (Math|Vector|BreakVector _array_element)))
            (:%20%20
              (Utilities|Array|Add (LocalVariables|GetInvertedPositions) (Math|Vector|MakeVector _result _result_2 (.Z (Math|Vector|BreakVector _array_element)))))))))
    (return (LocalVariables|GetInvertedPositions))
    (else
      (return InPositions))))

(fn PivotPositions
  (params (Direction :type Rotator) (InPositions :type Array%20of%20Vectors))
  (for (_array_element _array_index) InPositions
    (Utilities|IsValidIndex InPositions _array_index
      (:Valid
        (Utilities|Array|Add (LocalVariables|GetRotatedOffsets) (Math|Vector|RotateVector _array_element Direction)))))
  (return (LocalVariables|GetRotatedOffsets)))

(fn PivotPositionsatPoint
  (params (Direction :type Rotator) (Point :type Vector) (InPositions :type Array%20of%20Vectors))
  (bind _outpositions (CallFunction|PivotPositions Direction InPositions))
  (for _array_element _outpositions
    (Utilities|Array|Add (LocalVariables|GetAdjustedPivotPositions) (+ _array_element Point)))
  (return (LocalVariables|GetAdjustedPivotPositions)))

(fn PivotPositionswithDot
  (params (Direction :type Rotator) (Point :type Vector) (DotProduct :type Float%20%28double-precision%29))
  (Utilities|FlowControl|Sequence
    (:then_0
      (if (< DotProduct 0.0)
        (bind _outpositions (CallFunction|InvertPositions (Variables|Default|GetPositions)))
        (bind _output_get (Variables|Default|SetPositions _outpositions))
        (Variables|Default|SetPositionDecals _output_get)))
    (:then_1
      (bind _outpositions_2 (CallFunction|PivotPositionsatPoint Direction Point (Variables|Default|GetPositions)))
      (return _outpositions_2))))

(fn MoveCharacterstoPositions
  (params (Positions :type Array%20of%20Vectors))
  (for (_array_element _array_index) (Variables|Data|GetSquadMembers)
    (AI|Navigation|MovetoLocation (AI|GetAIController _array_element) (Utilities|Array|Get(acopy) Positions _array_index) 1.0 false true false true 0)))

(fn DrawPositionDecals
  (params (Point :type Vector))
  (bind (_cover _outpositions _class) (CallFunction|QueryAreaforCover Point (Utilities|GetSpacing)))
  (Utilities|IsValid _cover
    (:Is%20Valid
      (for _array_element _outpositions
        (if (Utilities|Enum|Equal(Enum) _class "NewEnumerator3")
          (Rendering|Debug|DrawDebugPoint _array_element 5.0 "(R=0.000000,G=1.000000,B=0.000000,A=1.000000)" 0.0)
          (else
            (Rendering|Debug|DrawDebugPoint _array_element 5.0 "(R=1.000000,G=0.450772,B=0.000000,A=1.000000)" 0.0)))))
    (:Is%20Not%20Valid
      (Utilities|FlowControl|Sequence
        (:then_0
          (if (< (Utilities|MovementDotProduct Point) 0.0)
            (bind _outpositions_2 (CallFunction|InvertPositions (Variables|Default|GetPositionDecals)))
            (Variables|Default|SetPositionDecals _outpositions_2)))
        (:then_1
          (bind _outpositions_3 (CallFunction|PivotPositionsatPoint (Math|Rotator|FindLookatRotation (Utilities|GetLeaderPosition) Point) Point (Variables|Default|GetPositionDecals)))
          (for _array_element_2 _outpositions_3
            (Rendering|Debug|DrawDebugPoint _array_element_2 5.0 "(R=1.000000,G=1.000000,B=1.000000,A=1.000000)" 0.0)))))))

(fn QueryAreaforCover
  (params (Point :type Vector) (Radius :type Float%20%28double-precision%29))
  (bind _projectedpositions (LocalVariables|GetProjectedPositions))
  ;[0.15 0.15 0.15 0.5] NOTE: This whole function should get refactored to get actual perimeter positions. This is 'close enough' for prototyping
  (Utilities|FlowControl|Sequence
    (:then_0
      ;;[0.15 0.15 0.15 0.5] Get the nearest cover
      (bind (_outactors _returnvalue) (Collision|SphereOverlapActors Point Radius (Utilities|Array|MakeArray "ObjectTypeQuery1" "ObjectTypeQuery2" "ObjectTypeQuery3" "ObjectTypeQuery4" "ObjectTypeQuery6" "ObjectTypeQuery5") "/SeinARTS_Framework/Blueprints/Cover/SAF_Cover.SAF_Cover_C"))
      (if _returnvalue
        (for _array_element _outactors
          (Utilities|IsValid (LocalVariables|GetNearestCover)
            (:Is%20Valid
              (if (> (Math|Vector|Distance(Vector) (Transformation|GetActorLocation (stale _output_get)) Point) (Math|Vector|Distance(Vector) (Transformation|GetActorLocation) Point))
                (LocalVariables|SetNearestCover (.AsSAF%20Cover (Utilities|Casting|CastToSAF_Cover _array_element)))))
            (:Is%20Not%20Valid
              (bind _output_get (LocalVariables|SetNearestCover (.AsSAF%20Cover (Utilities|Casting|CastToSAF_Cover _array_element)))))))
        (bind _assaf_cover_area (Utilities|Casting|CastToSAF_CoverArea (LocalVariables|GetNearestCover)))
        (if (Utilities|Enum|NotEqual(Enum) (Variables|/SeinARTS_Framework/Blueprints/Cover/SAF_CoverArea.SAF_CoverArea_C|GetCoverClass _assaf_cover_area) "NewEnumerator4")
          (for (_ _array_index) (Variables|Data|GetSquadMembers)
            (Utilities|Array|Add (LocalVariables|GetSpacedPositions) (+ Point (Math|Vector|RotateVector (* (Math|Vector|GetUnitDirection(Vector) Point (Transformation|GetActorLocation (LocalVariables|GetNearestCover))) (Utilities|GetSpacing)) (Math|Rotator|MakeRotator 0.0 0.0 (Math|Conversions|ToFloat(Integer) (* _array_index 45)))))))
          (return (LocalVariables|GetNearestCover) (LocalVariables|GetSpacedPositions) (Variables|/SeinARTS_Framework/Blueprints/Cover/SAF_CoverArea.SAF_CoverArea_C|GetCoverClass _assaf_cover_area)))
        (else
          (return 0 0 "NewEnumerator4"))))
    (:then_1
      (Utilities|IsValid (LocalVariables|GetNearestCover)
        (:Is%20Valid
          (for (_ _array_index_2) (Variables|Data|GetSquadMembers)
            (if (!= (Math|Integer|%(Integer) _array_index_2 2) 0)
              (LocalVariables|SetSpacingAlt (* (LocalVariables|GetSpacingItr) -1.0))
              (else
                (bind _output_get_2 (LocalVariables|SetSpacingItr (+ (LocalVariables|GetSpacingItr) (Utilities|GetSpacing))))
                (LocalVariables|SetSpacingAlt _output_get_2)))
            (bind _output_get_3 (LocalVariables|SetProjectionOffset (+ (* (Math|Vector|GetRightVector (Math|Rotator|FindLookatRotation (Transformation|GetActorLocation (LocalVariables|GetNearestCover)) (Math|Vector|MakeVector (.X (Math|Vector|BreakVector (+ (* (Math|Vector|GetUnitDirection(Vector) (Transformation|GetActorLocation (LocalVariables|GetNearestCover)) Point) (Utilities|GetSpacing) 2.0) Point))) (.Y (Math|Vector|BreakVector (+ (* (Math|Vector|GetUnitDirection(Vector) (Transformation|GetActorLocation (LocalVariables|GetNearestCover)) Point) (Utilities|GetSpacing) 2.0) Point))) (.Z (Math|Vector|BreakVector (Transformation|GetActorLocation (LocalVariables|GetNearestCover))))))) (LocalVariables|GetSpacingAlt)) (Math|Vector|MakeVector (.X (Math|Vector|BreakVector (+ (* (Math|Vector|GetUnitDirection(Vector) (Transformation|GetActorLocation (LocalVariables|GetNearestCover)) Point) (Utilities|GetSpacing) 2.0) Point))) (.Y (Math|Vector|BreakVector (+ (* (Math|Vector|GetUnitDirection(Vector) (Transformation|GetActorLocation (LocalVariables|GetNearestCover)) Point) (Utilities|GetSpacing) 2.0) Point))) (.Z (Math|Vector|BreakVector (Transformation|GetActorLocation (LocalVariables|GetNearestCover))))))))
            (bind _outhit (Collision|LineTraceByChannel _output_get_3 (Transformation|GetActorLocation (LocalVariables|GetNearestCover)) "TraceTypeQuery1" false 0 "None"))
            (Utilities|Array|Add (LocalVariables|GetProjectedPositions) (.ImpactPoint (Collision|BreakHitResult _outhit)))))))
    (:then_2
      ;;[0.15 0.15 0.15 0.5] All this does is add spacing between each projected position of at least (spacing). It uses direction vectors from projection point to projection point, which will mach the wrapping of the cover object. It resuses spacing itr and alt to amplify spacing
      (Utilities|IsNotEmpty (LocalVariables|GetProjectedPositions)
        (:True
          (for (_array_element_2 _array_index_3) (LocalVariables|GetProjectedPositions)
            (if (Utilities|Array|IsValidIndex _projectedpositions (- _array_index_3 1))
              (if (== (LocalVariables|GetSpacingItr) (LocalVariables|GetSpacingAlt))
                (Math|Float|NegateFloat (LocalVariables|GetSpacingAlt)
                  (:%20%20
                    _))
                (else
                  (LocalVariables|SetSpacingAlt (LocalVariables|GetSpacingItr))))
              (Utilities|Array|Add (LocalVariables|GetSpacedPositions) (.ProjectedLocation (AI|Navigation|ProjectPointtoNavigation (+ _array_element_2 (* (Math|Vector|GetUnitDirection(Vector) (Utilities|Array|Get(acopy) _projectedpositions (- _array_index_3 1)) _array_element_2) (LocalVariables|GetSpacingItr))) 0 0 "100.000000,100.000000,100.000000")))
              (Rendering|Debug|DrawDebugPoint (.ProjectedLocation (AI|Navigation|ProjectPointtoNavigation (+ _array_element_2 (* (Math|Vector|GetUnitDirection(Vector) (Utilities|Array|Get(acopy) _projectedpositions (- _array_index_3 1)) _array_element_2) (LocalVariables|GetSpacingItr))) 0 0 "100.000000,100.000000,100.000000")) 5.0 "(R=0.000000,G=1.000000,B=0.000000,A=1.000000)" 0.0)
              (if (== (* (LocalVariables|GetSpacingAlt) -1.0) (LocalVariables|GetSpacingItr))
                (LocalVariables|SetSpacingItr (* (LocalVariables|GetSpacingItr) 2.0))
                (LocalVariables|SetSpacingAlt (* (LocalVariables|GetSpacingAlt) 2.0)))
              (else
                (LocalVariables|SetSpacingItr (Utilities|GetSpacing))
                (LocalVariables|SetSpacingAlt 0.0)
                (Utilities|Array|Add (LocalVariables|GetSpacedPositions) (.ProjectedLocation (AI|Navigation|ProjectPointtoNavigation _array_element_2 0 0 "100.000000,100.000000,100.000000")))))))))
    (:then_3
      (return (LocalVariables|GetNearestCover) (LocalVariables|GetSpacedPositions) (Variables|/SeinARTS_Framework/Blueprints/Cover/SAF_Cover.SAF_Cover_C|GetCoverClass (LocalVariables|GetNearestCover))))))

(fn GetNearestTarget
  (params (Position :type Vector))
  (for _array_element (Variables|Default|GetAllTargets)
    (Utilities|IsValid (LocalVariables|GetNearestTarget)
      (:Is%20Valid
        (if (< (Math|Vector|Distance(Vector) (Transformation|GetActorLocation _array_element) Position) (Math|Vector|Distance(Vector) (Transformation|GetActorLocation (LocalVariables|GetNearestTarget)) Position))
          (LocalVariables|SetNearestTarget _array_element)))
      (:Is%20Not%20Valid
        (LocalVariables|SetNearestTarget _array_element))))
  (return (LocalVariables|GetNearestTarget)))

(fn GetAmmo
  (return (Variables|Default|GetAmmo)))

(fn GetAmmo%
  (return (/ (Variables|Default|GetAmmo) (Variables|/SeinARTS_Framework/Blueprints/Data/SAFD_Unit.SAFD_Unit_C|GetAmmo (Variables|Data|GetUnitData)))))

(fn GetHP
  (for _array_element (Variables|Data|GetSquadMembers)
    (bind _hp (Default|GetHP _array_element))
    (LocalVariables|SetCummulativeHP (+ _hp (LocalVariables|GetCummulativeHP))))
  (return (LocalVariables|GetCummulativeHP)))

(fn GetHP%
  (for _array_element (Variables|Data|GetSquadMembers)
    (LocalVariables|SetCummulativeMaxHP (+ (Variables|/SeinARTS_Framework/Blueprints/Data/SAFD_SquadMember.SAFD_SquadMember_C|GetHP (Variables|/SeinARTS_Framework/Blueprints/Units/SAF_SquadMember.SAF_SquadMember_C|GetSquadMemberData _array_element)) (LocalVariables|GetCummulativeMaxHP))))
  (bind _hp (CallFunction|GetHP))
  (return (/ _hp (LocalVariables|GetCummulativeMaxHP))))

(fn GetMF
  (return (Variables|Default|GetMorale)))

(fn GetMF%
  (return (/ (Variables|Default|GetMorale) (Variables|/SeinARTS_Framework/Blueprints/Data/SAFD_Squad.SAFD_Squad_C|GetMorale (Variables|Data|GetSquadData)))))

(fn GetPlayerOwner
  (return (Variables|Data|GetPlayerOwner)))

(fn GetUnitData
  (return (Variables|Data|GetUnitData) (Variables|Data|GetInstanceID)))

(fn Order
  (params (Target :type Actor%20Object%20Reference) (Position :type Vector :default "0, 0, 0"))
  (Utilities|IsValid Target
    (:Is%20Valid
      (CallFunction|ReceiveTarget 0 true))
    (:Is%20Not%20Valid
      (bind (_cover _outpositions) (CallFunction|QueryAreaforCover Position (Utilities|GetSpacing)))
      (Utilities|IsValid _cover
        (:Is%20Valid
          (CallFunction|MoveCharacterstoPositions _outpositions))
        (:Is%20Not%20Valid
          (bind _outpositions_2 (CallFunction|PivotPositionswithDot (Math|Rotator|FindLookatRotation (Utilities|GetLeaderPosition) Position) Position (Utilities|MovementDotProduct Position)))
          (CallFunction|MoveCharacterstoPositions _outpositions_2)))
      (return true))))

(fn ProvideTarget
  (params (Requestor :type Actor%20Object%20Reference))
  (bind _activetarget (Variables|Default|GetActiveTarget))
  (Utilities|IsValid _activetarget
    (:Is%20Valid
      (return _activetarget))
    (:Is%20Not%20Valid
      (bind _target (CallFunction|GetNearestTarget (Transformation|GetActorLocation Requestor)))
      (return _target))))

(fn QueueSelect
  (bind _output_get (Variables|Selection|SetSelectQueued (Variables|Selection|GetSelectable)))
  (return _output_get self))

(fn Select
  (bind _output_get (Variables|Selection|SetSelected (Variables|Selection|GetSelectable)))
  (return _output_get self))