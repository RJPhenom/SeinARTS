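; Player controller for SeinARTS RTS-style play that translates Enhanced Input into selection, order, ping and camera controls.
; On BeginPlay it adds the SAF input mapping context and caches the camera pawn, which receives pan, rotate, zoom, speed-toggle and reset inputs.
; Select, Order and Ping actions pass mouse position to start, update and end handlers, modifier queries expose Shift/Control/Alt state, and Q sends a test squad move order.
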(event Input|EnhancedActionEvents|EnhancedInputActionSAF_IA-Order
  (params (ActionValue :type Boolean) (ElapsedSeconds :type Float%20%28double-precision%29) (TriggeredSeconds :type Float%20%28double-precision%29) (InputAction :type Input%20Action%20Object%20Reference :default "/SeinARTS_Framework/Blueprints/Input/SAF_IA-Order.SAF_IA-Order"))
  (bind _returnvalue (Class|SAFPlayerController|GetMouseVector2D))
  (:Triggered
    (Class|SAFPlayerInterface|OnOrderUpdatedHandler _returnvalue))
  (:Started
    (Default|CallOnOrderStarted _returnvalue))
  (:Canceled
    (Default|CallOnOrderEnded _returnvalue :!label _label))
  (:Completed
    (goto _label)))

(event Input|EnhancedActionEvents|EnhancedInputActionSAF_IA-Ping
  (params (ActionValue :type Boolean) (ElapsedSeconds :type Float%20%28double-precision%29) (TriggeredSeconds :type Float%20%28double-precision%29) (InputAction :type Input%20Action%20Object%20Reference :default "/SeinARTS_Framework/Blueprints/Input/SAF_IA-Ping.SAF_IA-Ping"))
  (bind _returnvalue (Class|SAFPlayerController|GetMouseVector2D))
  (:Triggered
    (Class|SAFPlayerInterface|OnPingUpdatedHandler _returnvalue))
  (:Started
    (Default|CallOnPingStarted _returnvalue))
  (:Canceled
    (Default|CallOnPingEnded _returnvalue :!label _label))
  (:Completed
    (goto _label)))

(event Input|EnhancedActionEvents|EnhancedInputActionSAF_IA-Pan
  (params (ActionValue :type Vector%202D%20Structure) (ElapsedSeconds :type Float%20%28double-precision%29) (TriggeredSeconds :type Float%20%28double-precision%29) (InputAction :type Input%20Action%20Object%20Reference :default "/SeinARTS_Framework/Blueprints/Input/SAF_IA-Pan.SAF_IA-Pan"))
  (Class|SAFCameraPawn|PanCamera (Variables|Default|GetAs%20SAFBPCamera%20Pawn) ActionValue))

(event Input|EnhancedActionEvents|EnhancedInputActionSAF_IA-Select
  (params (ActionValue :type Boolean) (ElapsedSeconds :type Float%20%28double-precision%29) (TriggeredSeconds :type Float%20%28double-precision%29) (InputAction :type Input%20Action%20Object%20Reference :default "/SeinARTS_Framework/Blueprints/Input/SAF_IA-Select.SAF_IA-Select"))
  (bind _returnvalue (Class|SAFPlayerController|GetMouseVector2D))
  (:Triggered
    (Class|SAFPlayerInterface|OnSelectUpdatedHandler _returnvalue))
  (:Started
    (Default|CallOnSelectStarted _returnvalue))
  (:Canceled
    (Default|CallOnSelectEnded _returnvalue :!label _label))
  (:Completed
    (goto _label)))

(event Input|EnhancedActionEvents|EnhancedInputActionSAF_IA-Zoom
  (params (ActionValue :type Float%20%28double-precision%29) (ElapsedSeconds :type Float%20%28double-precision%29) (TriggeredSeconds :type Float%20%28double-precision%29) (InputAction :type Input%20Action%20Object%20Reference :default "/SeinARTS_Framework/Blueprints/Input/SAF_IA-Zoom.SAF_IA-Zoom"))
  (Class|SAFCameraPawn|ZoomCamera (Variables|Default|GetAs%20SAFBPCamera%20Pawn) ActionValue))

(event Input|EnhancedActionEvents|EnhancedInputActionSAF_IA-Rotate
  (params (ActionValue :type Vector%202D%20Structure) (ElapsedSeconds :type Float%20%28double-precision%29) (TriggeredSeconds :type Float%20%28double-precision%29) (InputAction :type Input%20Action%20Object%20Reference :default "/SeinARTS_Framework/Blueprints/Input/SAF_IA-Rotate.SAF_IA-Rotate"))
  (Class|SAFCameraPawn|RotateCamera (Variables|Default|GetAs%20SAFBPCamera%20Pawn) ActionValue))

(event Input|EnhancedActionEvents|EnhancedInputActionSAF_IA-Follow
  (params (ActionValue :type Boolean) (ElapsedSeconds :type Float%20%28double-precision%29) (TriggeredSeconds :type Float%20%28double-precision%29) (InputAction :type Input%20Action%20Object%20Reference :default "/SeinARTS_Framework/Blueprints/Input/SAF_IA-Follow.SAF_IA-Follow")))

(event Input|EnhancedActionEvents|EnhancedInputActionSAF_IA-Shift
  (params (ActionValue :type Boolean) (ElapsedSeconds :type Float%20%28double-precision%29) (TriggeredSeconds :type Float%20%28double-precision%29) (InputAction :type Input%20Action%20Object%20Reference :default "/SeinARTS_Framework/Blueprints/Input/SAF_IA-Shift.SAF_IA-Shift"))
  (:Started
    (Class|SAFCameraPawn|ToggleSpeed (Variables|Default|GetAs%20SAFBPCamera%20Pawn) ActionValue :!label _label))
  (:Canceled
    (goto _label))
  (:Completed
    (goto _label)))

(event Input|EnhancedActionEvents|EnhancedInputActionSAF_IA-Reset
  (params (ActionValue :type Boolean) (ElapsedSeconds :type Float%20%28double-precision%29) (TriggeredSeconds :type Float%20%28double-precision%29) (InputAction :type Input%20Action%20Object%20Reference :default "/SeinARTS_Framework/Blueprints/Input/SAF_IA-Reset.SAF_IA-Reset"))
  (:Completed
    (Class|SAFCameraPawn|ResetCamera (Variables|Default|GetAs%20SAFBPCamera%20Pawn))))

(event Input|EnhancedActionEvents|EnhancedInputActionSAF_IA-Q
  (params (ActionValue :type Boolean) (ElapsedSeconds :type Float%20%28double-precision%29) (TriggeredSeconds :type Float%20%28double-precision%29) (InputAction :type Input%20Action%20Object%20Reference :default "/SeinARTS_Framework/Blueprints/Input/SAF_IA-Q.SAF_IA-Q"))
  (:Started
    (Class|SAFPlayerInterface|SendOrder (Utilities|Struct|MakeSAFOrder 0 "/SeinARTS_Framework/Blueprints/Data/TestSquadData.TestSquadData" "0.000000,0.000000,0.000000" "0.000000,0.000000,0.000000" "(TagName=\"SeinARTS.Order.Move\")") false)))

(event EventBeginPlay
  (bind _returnvalue (PlayerController|LocalPlayerSubsystems|GetEnhancedInputLocalPlayerSubsystem))
  ;[0.15 0.15 0.15 0.5] Init Input Sys
  (Utilities|IsValid _returnvalue
    (:Is%20Valid
      (Input|AddMappingContext _returnvalue "/SeinARTS_Framework/Blueprints/Input/SAF_IMAP.SAF_IMAP" 0 "(bIgnoreAllPressedKeysUntilRelease=True,bForceImmediately=False,bNotifyUserSettings=False)")
      (bind _assafbpcamera_pawn (Utilities|Casting|CastToSAFBPCameraPawn (Pawn|GetControlledPawn)))
      (Variables|Default|SetAs%20SAFBPCamera%20Pawn _assafbpcamera_pawn))))

(fn ConstructionScript)

(fn IsQueueButtonDown
  (return (Input|EnhancedActionValues|GetSAF_IA-Shift)))

(fn IsControlButtonDown
  (return (Input|EnhancedActionValues|GetSAF_IA-Control)))

(fn IsAlternateButtonDown
  (return (Input|EnhancedActionValues|GetSAF_IA-Alt)))