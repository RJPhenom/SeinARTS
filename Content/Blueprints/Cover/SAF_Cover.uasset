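; SAF_Cover is a cover actor that puts squad members into and out of cover through its box trigger.
; On begin and end overlap it calls EnterCover or ExitCover on the SAF_SquadMember, passing itself and its CoverClass.
; Entering also passes a direction from GetDirection, a unit vector from the cover to a given actor, though the overlap event leaves that actor input unset.
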(event OnComponentBeginOverlap(Box)
  (params (OverlappedComponent :type Primitive%20Component%20Object%20Reference) (OtherActor :type Actor%20Object%20Reference) (OtherComp :type Primitive%20Component%20Object%20Reference) (OtherBodyIndex :type Integer) (bFromSweep :type Boolean) (SweepResult :type Hit%20Result%20Structure%20%28by%20ref%29))
  (bind _assaf_squad_member (Utilities|Casting|CastToSAF_SquadMember OtherActor))
  (bind _direction (CallFunction|GetDirection))
  (Default|EnterCover _assaf_squad_member self (Variables|Default|GetCoverClass) _direction))

(event OnComponentEndOverlap(Box)
  (params (OverlappedComponent :type Primitive%20Component%20Object%20Reference) (OtherActor :type Actor%20Object%20Reference) (OtherComp :type Primitive%20Component%20Object%20Reference) (OtherBodyIndex :type Integer))
  (bind _assaf_squad_member (Utilities|Casting|CastToSAF_SquadMember OtherActor))
  (Default|ExitCover _assaf_squad_member self (Variables|Default|GetCoverClass)))

(event EventBeginPlay)

(event Collision|EventActorBeginOverlap
  (params (OtherActor :type Actor%20Object%20Reference)))

(event EventTick
  (params (DeltaSeconds :type Float%20%28single-precision%29)))

(fn ConstructionScript)

(fn GetDirection
  (params (Actor :type Actor%20Object%20Reference))
  (return (Math|Vector|GetUnitDirection(Vector) (Transformation|GetActorLocation) (Transformation|GetActorLocation Actor))))